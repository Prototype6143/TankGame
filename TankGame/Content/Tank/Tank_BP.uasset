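; Tank Blueprint that handles component setup and orbit camera controls for the player tank.
; On BeginPlay it passes the barrel and turret components to SetTankComponentsReference.
; Camera axis inputs yaw the Scene component and pitch the SpringArm separately, scaled by delta time.
; Zoom actions step the SpringArm's target length by ZoomValue, with no clamping.
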(event `self.ReceiveBeginPlay`
  (`self.SetTankComponentsReference` (`self.TankBarrel`) (`self.TankTurret`)))

(event `InputAxis|CameraRotationX`
  (params (AxisValue :type "Float (single-precision)"))
  ;[1 1 1] Set Camera rotation axis
  (`SceneComponent.K2_AddLocalRotation` (`self.Scene`) (`KismetMathLibrary.MakeRotator` 0.0 0.0 (* AxisValue (`GameplayStatics.GetWorldDeltaSeconds`) 100.0)) false false))

(event `InputAxis|CameraRotationY`
  (params (AxisValue :type "Float (single-precision)"))
  ;[1 1 1] Set Camera rotation axis
  (`SceneComponent.K2_AddLocalRotation` (`self.SpringArm`) (`KismetMathLibrary.MakeRotator` 0.0 (* AxisValue (`GameplayStatics.GetWorldDeltaSeconds`) 100.0)) false false))

(event `InputAction|ZoomIn`
  (params (Key :type "Key Structure" :default "AnyKey"))
  (bind _springarm (`self.SpringArm`))
  ;[1 1 1] Set Zoom distance from the player tank
  (:`Pressed`
    (set `SpringArmComponent.TargetArmLength` (- (`SpringArmComponent.TargetArmLength` _springarm) (`self.ZoomValue`)) _springarm)))

(event `InputAction|ZoomOut`
  (params (Key :type "Key Structure" :default "AnyKey"))
  (bind _springarm (`self.SpringArm`))
  ;[1 1 1] Set Zoom distance from the player tank
  (:`Pressed`
    (set `SpringArmComponent.TargetArmLength` (+ (`SpringArmComponent.TargetArmLength` _springarm) (`self.ZoomValue`)) _springarm)))

(fn `UserConstructionScript`)